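; InventoryHUD is an actor Blueprint that owns the player's inventory screen, creating the InventoryWidget hidden in the viewport on BeginPlay.
; A toggle function shows or hides it, switching the first player controller between game-and-UI and game-only input and setting cursor visibility.
; The widget's item list refreshes whenever the screen opens, and a separate update function exposes that refresh directly.
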(event `self.ReceiveBeginPlay`
  (bind _returnvalue (`|CreateWidget` "/Game/Blueprints/HUD/InventoryWidget.InventoryWidget_C"))
  (bind _output_get (set `self.InventoryUI` _returnvalue))
  (`UserWidget.AddToViewport` _output_get 0)
  (`Widget.SetVisibility` _output_get "Hidden"))

(fn `HideInventoryScreen`
  (`Widget.SetVisibility` (`self.InventoryUI`) "Hidden")
  (`WidgetBlueprintLibrary.SetInputMode_GameOnly` (`GameplayStatics.GetPlayerController` 0)))

(fn `ShowInventoryScreen`
  (bind _inventoryui (`self.InventoryUI`))
  (`Widget.SetVisibility` _inventoryui "Visible")
  (`WidgetBlueprintLibrary.SetInputMode_GameAndUIEx` (`GameplayStatics.GetPlayerController` 0) _inventoryui "DoNotLock" false)
  (`/Game/Blueprints/HUD/InventoryWidget.UpdateList` _inventoryui))

(fn `ToggleInventoryScreen`
  (bind _returnvalue (`GameplayStatics.GetPlayerController` 0))
  (if (`|EnumEquality` (`Widget.GetVisibility` (`self.InventoryUI`)) "Visible")
    (`self.HideInventoryScreen`)
    (set `PlayerController.bShowMouseCursor` false _returnvalue)
    (else
      (`self.ShowInventoryScreen`)
      (set `PlayerController.bShowMouseCursor` true _returnvalue))))

(fn `UpdateInventoryWidget`
  (`/Game/Blueprints/HUD/InventoryWidget.UpdateList` (`self.InventoryUI`)))

(fn `UserConstructionScript`)