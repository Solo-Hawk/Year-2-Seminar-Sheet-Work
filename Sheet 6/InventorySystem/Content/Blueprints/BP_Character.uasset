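; Player character Blueprint with camera-relative planar movement, look input and item pickup into an inventory.
; Interact/Pickup runs a debug-drawn box trace forward from the camera and passes any hit CPP_ItemBase actor to InventoryComponent.
; BeginPlay binds the component's list-update event so the InventoryHUD refreshes its widget, and GetInventory exposes the component's inventory.
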(event `self.ReceiveBeginPlay`
  (add `/Game/Blueprints/InventorySystem/InventoryComponent.UpdateList` (`self.InventoryComponent`) (delegate `UpdateInventoryUI`)))

(event `UpdateInventoryUI`
  (bind _asinventory_hud (cast `/Game/Blueprints/HUD/InventoryHUD` (`PlayerController.GetHUD` (`GameplayStatics.GetPlayerController` 0))))
  (`/Game/Blueprints/HUD/InventoryHUD.UpdateInventoryWidget` _asinventory_hud))

(event `self.ReceiveActorBeginOverlap`
  (params (OtherActor :type "Actor Object Reference")))

(event `InputAxis|Look_Up`
  (params (AxisValue :type "Float (single-precision)"))
  ;[1 1 1] Movement
  (`self.AddControllerPitchInput` AxisValue))

(event `InputAxis|Move_Forward`
  (params (AxisValue :type "Float (single-precision)"))
  ;[1 1 1] Movement
  (`self.AddMovementInput` (`KismetMathLibrary.GetForwardVector` (`KismetMathLibrary.MakeRotator` 0.0 0.0 (.yaw (`self.GetControlRotation`)))) AxisValue))

(event `InputAxis|Look_Right`
  (params (AxisValue :type "Float (single-precision)"))
  ;[1 1 1] Movement
  (`self.AddControllerYawInput` AxisValue))

(event `InputAxis|Move_Right`
  (params (AxisValue :type "Float (single-precision)"))
  ;[1 1 1] Movement
  (`self.AddMovementInput` (`KismetMathLibrary.GetRightVector` (`KismetMathLibrary.MakeRotator` 0.0 0.0 (.yaw (`self.GetControlRotation`)))) AxisValue))

(event `InputAction|Interact/Pickup`
  (params (Key :type "Key Structure"))
  (bind _camera (`self.Camera`))
  (bind _returnvalue (`SceneComponent.K2_GetComponentLocation` _camera))
  (:`Pressed`
    (bind (_outhit _returnvalue_2) (`KismetSystemLibrary.BoxTraceSingleForObjects` :`Start` _returnvalue :`End` (+ _returnvalue (* (`SceneComponent.GetForwardVector` _camera) 600.0)) :`HalfSize` (20.0 20.0 20.0) :`Orientation` (`SceneComponent.K2_GetComponentRotation` _camera) :`ObjectTypes` (`|MakeArray` "ObjectTypeQuery2" :!type "EObjectTypeQuery Enum") :`DrawDebugType` "ForDuration" :`DrawTime` 2.0))
    (if _returnvalue_2
      (bind _ascpp_item_base (cast `CPP_ItemBase` (`.HitActor` (`GameplayStatics.BreakHitResult` _outhit))))
      (`/Game/Blueprints/InventorySystem/InventoryComponent.AddItem` (`self.InventoryComponent`) _ascpp_item_base))))

(fn `GetInventory`
  (returns (Inventory :type "Array of /Game/Blueprints/InventorySystem/ItemStack Structure"))
  (return (`/Game/Blueprints/InventorySystem/InventoryComponent.Inventory` (`self.InventoryComponent`))))

(fn `UserConstructionScript`)