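; Inventory component that stores items as an array of name, stack, max stack, index and class-reference structs.
; AddItem tops up a non-full stack of the same name or appends a new one, while RemoveItem decrements stacks and returns the class.
; DropItem spawns that class in front of the player.
; SplitStack halves a stack, FillStack merges a matching one into the selected slot, and changes trigger CallUpdateList.
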(fn `AddItem`
  (params (Item :type "CPP_ItemBase Object Reference"))
  (locals (PickupItem :type "CPP_ItemBase Object Reference") (CurrentStack :type "/Game/Blueprints/InventorySystem/ItemStack Structure") (CurrentIndex :type Integer))
  (bind _pickupitem (`local.PickupItem`))
  (bind _inventory (`self.Inventory`))
  (bind (_name _stack _maxstack _index _classreference) (break `/Game/Blueprints/InventorySystem/ItemStack` (`local.CurrentStack`)))
  (bind _output_get (set `local.PickupItem` Item))
  (for (_array_element _array_index) (`self.Inventory`)
    (set `local.CurrentIndex` _array_index)
    (set `local.CurrentStack` _array_element)
    (bind (_name_2 _stack_2 _maxstack_2) (break `/Game/Blueprints/InventorySystem/ItemStack` _array_element))
    (if (`KismetStringLibrary.EqualEqual_StrStr` _name_2 (`CPP_ItemBase.Name` (`local.PickupItem`)))
      (if (not (== _stack_2 _maxstack_2))
        (bind _result (`/Engine/EditorBlueprintResources/StandardMacros.IncrementInt` _stack)
          (:`  `
            (`KismetArrayLibrary.Array_Set` (`self.Inventory`) (`local.CurrentIndex`) (make `/Game/Blueprints/InventorySystem/ItemStack` _name _result _maxstack _index _classreference) true)
            (`CPP_ItemBase.PickupItem` (`local.PickupItem`))
            (`self.UpdateList`)
            (return))))))
  (bind _returnvalue (`KismetArrayLibrary.Array_Add` _inventory (make `/Game/Blueprints/InventorySystem/ItemStack` "")))
  (bind _returnvalue_2 (`GameplayStatics.GetObjectClass` _output_get))
  (`KismetArrayLibrary.Array_Set` _inventory _returnvalue (make `/Game/Blueprints/InventorySystem/ItemStack` (`CPP_ItemBase.Name` _pickupitem) 1 50 _returnvalue _returnvalue_2) true)
  (`CPP_ItemBase.PickupItem` _pickupitem)
  (`KismetSystemLibrary.PrintString` (`KismetStringLibrary.Concat_StrStr` "New Item:" (`KismetSystemLibrary.GetClassDisplayName` _returnvalue_2)))
  (`self.UpdateList`)
  (return))

(fn `DropItem`
  (params (Name :type String))
  (bind _returnvalue (`GameplayStatics.GetPlayerCharacter` 0))
  (bind _itemclassreference (`self.RemoveItem` Name))
  (`|SpawnActorFromClass` _itemclassreference (`KismetMathLibrary.Conv_VectorToTransform` (+ (* (`Actor.GetActorForwardVector` _returnvalue) 300.0) (`SceneComponent.K2_GetComponentLocation` (`Character.Mesh` _returnvalue)))) "Undefined" "OverrideRootScale" null null))

(fn `FillStack`
  (params (Index :type Integer))
  (locals (StackIndex :type Integer) (`Current Stack` :type "/Game/Blueprints/InventorySystem/ItemStack Structure") (NewStackSize :type Integer))
  (bind _inventory (`self.Inventory`))
  (bind _inventory_2 (`self.Inventory`))
  (bind _stackindex (`local.StackIndex`))
  (bind (_name _stack _maxstack _index _classreference) (break `/Game/Blueprints/InventorySystem/ItemStack` (`local.Current Stack`)))
  (bind (_name_2 _stack_2 _maxstack_2 _index_2 _classreference_2) (break `/Game/Blueprints/InventorySystem/ItemStack` (`|GetArrayItem` _inventory Index)))
  (set `local.StackIndex` Index)
  (for (_array_element _array_index) _inventory
    (bind _output_get (set `local.Current Stack` _array_element))
    (if (!= _array_index Index)
      (bind (_name_3 _stack_3 _maxstack_3) (break `/Game/Blueprints/InventorySystem/ItemStack` _output_get))
      (if (and (!= _stack_3 _maxstack_3) (`KismetStringLibrary.EqualEqual_StrStr` _name_3 _name_2))
        (bind _returnvalue (+ _stack_3 _stack_2))
        (if (not (> _returnvalue _maxstack_2))
          (`KismetArrayLibrary.Array_Set` _inventory_2 _stackindex (make `/Game/Blueprints/InventorySystem/ItemStack` _name_2 _returnvalue _maxstack_2 _index_2 _classreference_2) true)
          (`KismetArrayLibrary.Array_Remove` _inventory_2 _index)
          (else
            (set `local.NewStackSize` (- _returnvalue _maxstack_2))
            (`KismetArrayLibrary.Array_Set` _inventory_2 _stackindex (make `/Game/Blueprints/InventorySystem/ItemStack` _name_2 _maxstack_2 _maxstack_2 _index_2 _classreference_2) true)
            (`KismetArrayLibrary.Array_Set` _inventory_2 _index (make `/Game/Blueprints/InventorySystem/ItemStack` _name (`local.NewStackSize`) _maxstack _index _classreference) true)))
        (`self.UpdateList`)
        (return)))))

(fn `RemoveItem`
  (params (ItemName :type String))
  (returns (ItemClassReference :type "CPP_ItemBase Class Reference"))
  (locals (Name :type String) (CurrentIndex :type Integer) (CurrentStack :type "/Game/Blueprints/InventorySystem/ItemStack Structure"))
  (bind _inventory (`self.Inventory`))
  (bind _currentindex (`local.CurrentIndex`))
  (bind (_name _stack _maxstack _index _classreference) (break `/Game/Blueprints/InventorySystem/ItemStack` (`local.CurrentStack`)))
  (set `local.Name` ItemName)
  (for (_array_element _array_index) (`self.Inventory`)
    (set `local.CurrentStack` _array_element)
    (set `local.CurrentIndex` _array_index)
    (if (`KismetStringLibrary.EqualEqual_StrStr` (`local.Name`) _name)
      (bind _result (`/Engine/EditorBlueprintResources/StandardMacros.DecrementInt` _stack)
        (:`  `
          (if (== _result 0)
            (`KismetArrayLibrary.Array_Remove` _inventory _currentindex)
            (else
              (`KismetArrayLibrary.Array_Set` _inventory _currentindex (make `/Game/Blueprints/InventorySystem/ItemStack` _name _result _maxstack _index _classreference) true)))
          (`self.UpdateList`)
          (return _classreference))))))

(fn `SplitStack`
  (params (Index :type Integer))
  (locals (StackIndex :type Integer))
  (bind _inventory (`self.Inventory`))
  (bind _output_get (set `local.StackIndex` Index))
  (bind _returnvalue (`KismetArrayLibrary.Array_Add` _inventory))
  (bind (_name _stack _maxstack _index _classreference) (break `/Game/Blueprints/InventorySystem/ItemStack` (`|GetArrayItem` _inventory _output_get)))
  (`KismetArrayLibrary.Array_Set` _inventory _returnvalue (make `/Game/Blueprints/InventorySystem/ItemStack` _name (+ (mod _stack 2) (/ _stack 2)) _maxstack _returnvalue _classreference))
  (`KismetArrayLibrary.Array_Set` _inventory _index (make `/Game/Blueprints/InventorySystem/ItemStack` _name (/ _stack 2) _maxstack _index _classreference))
  (`self.UpdateList`))