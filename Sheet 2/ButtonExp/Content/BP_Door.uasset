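; BP_Door is a double door that toggles open and closed through an interact event.
; The DoorSwing timeline yaws two scene components in opposite directions, playing from start or reversing from end based on IsOpen, then inverts that flag.
; BeginPlay runs the same toggle once, and each trigger restarts the swing from an endpoint rather than its current position.
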(event `self.ReceiveBeginPlay`
  (bind _isopen (`self.isOpen`))
  (`|ExecutionSequence` :!label _label
    (:`then_0`
      (if _isopen
        (bind (_direction _curve) (`Timeline|DoorSwing` :!via `PlayFromStart` :!label _label_2)
          (:`Update`
            (`|ExecutionSequence`
              (:`then_0`
                (`SceneComponent.K2_SetRelativeRotation` (`self.Scene`) (`KismetMathLibrary.MakeRotator` 0.0 0.0 _curve) false false))
              (:`then_1`
                (`SceneComponent.K2_SetRelativeRotation` (`self.Scene1`) (`KismetMathLibrary.MakeRotator` 0.0 0.0 (* _curve -1.0)) false false)))))
        (else
          (goto _label_2 :!via `ReverseFromEnd`))))
    (:`then_1`
      (set `self.isOpen` (not _isopen)))))

(event `interact_Event`
  (goto _label))

(fn `UserConstructionScript`)