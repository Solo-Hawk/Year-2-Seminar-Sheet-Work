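; BP_Button is an interactable toggle button that triggers an InteractEvent on its Target and animates its Sphere component.
; BeginPlay caches the Sphere's relative position as the rest point.
; Each interact_Event flips IsToggle, notifies Target, then plays the MoveGraph timeline forward or in reverse.
; The timeline's scaled ButtonShift track offsets the Sphere along local X from that cached position.
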(event `self.ReceiveBeginPlay`
  (set `self.OriginalPosition` (`KismetMathLibrary.TransformLocation` (`SceneComponent.GetRelativeTransform` (`self.Sphere`)))))

(event `interact_Event`
  (bind _output_get (set `self.isToggle` (not (`self.isToggle`))))
  (`/Game/BP_Door.interact_Event` (`self.Target`))
  (if _output_get
    (bind (_direction _buttonshift) (`Timeline|MoveGraph` :!via `PlayFromStart` :!label _label)
      (:`Update`
        (`SceneComponent.K2_SetRelativeLocation` (`self.Sphere`) (+ (`self.OriginalPosition`) (`KismetMathLibrary.MakeVector` (* _buttonshift 10.0))) false false)))
    (else
      (goto _label :!via `ReverseFromEnd`))))

(fn `UserConstructionScript`)